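; Third-person shooter player character with Enhanced Input movement, look, jump, run and switching between a handgun and a sniper rifle.
; ChangeWeapon toggles mesh visibility and the flag that routes firing.
; Both guns spawn BP_Bullet from sockets with sound and camera shake.
; The sniper also line-traces from the camera for explosions, BP_EnemyFSM damage or physics impulses, and has a scope UI with narrowed FOV.
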(event Input|EnhancedActionEvents|EnhancedInputActionIA_Fire
  (params (ActionValue :type Boolean) (ElapsedSeconds :type Float%20%28double-precision%29) (TriggeredSeconds :type Float%20%28double-precision%29) (InputAction :type Input%20Action%20Object%20Reference :default "/Game/Input/IA_Fire.IA_Fire"))
  (bind _returnvalue (Game|GetPlayerController 0))
  (bind _playercameramanager (Variables|/Script/Engine.PlayerController|GetPlayerCameraManager _returnvalue))
  (bind _returnvalue_2 (Transformation|GetActorLocation _playercameramanager))
  (:Started
    (Utilities|FlowControl|Sequence
      (:then_0
        (if (Variables|Default|GetbUsing%20HandGun)
          (CallFunction|HandGunFire)
          (else
            (CallFunction|SniperFire)
            (bind (_outhit _returnvalue_3) (Collision|LineTraceByChannel _returnvalue_2 (+ _returnvalue_2 (* (Transformation|GetActorForwardVector _playercameramanager) 1e+05)) "TraceTypeQuery1" false 0 "None"))
            (if _returnvalue_3
              (Effects|SpawnEmitteratLocation "/Game/StarterContent/Particles/P_Explosion.P_Explosion" (.ImpactPoint (Collision|BreakHitResult _outhit)))
              (Utilities|IsValid (Actor|GetComponentbyClass (.HitActor (Collision|BreakHitResult _outhit)) "/Game/Blueprint/BP_EnemyFSM.BP_EnemyFSM_C")
                (:Is%20Valid
                  (Default|OnDamageProcess (Actor|GetComponentbyClass (.HitActor (Collision|BreakHitResult _outhit)) "/Game/Blueprint/BP_EnemyFSM.BP_EnemyFSM_C")))
                (:Is%20Not%20Valid
                  (if (Physics|IsSimulatingPhysics (.HitComponent (Collision|BreakHitResult _outhit)) "None")
                    (Class|PrimitiveComponent|AddForceatLocation (.HitComponent (Collision|BreakHitResult _outhit)) (* (Transformation|GetActorForwardVector) 1e+05) (.TraceEnd (Collision|BreakHitResult _outhit)) "None"))))))))
      (:then_1
        (CameraShakes|StartCameraShake (Game|GetPlayerCameraManager 0) "/Game/Blueprint/BP_CameraShake.BP_CameraShake_C" 1.0 "CameraLocal" "0, 0, 0")))))

(event Input|EnhancedActionEvents|EnhancedInputActionIA_SniperUI
  (params (ActionValue :type Boolean) (ElapsedSeconds :type Float%20%28double-precision%29) (TriggeredSeconds :type Float%20%28double-precision%29) (InputAction :type Input%20Action%20Object%20Reference :default "/Game/Input/IA_SniperUI.IA_SniperUI"))
  (bind _sniperui (Variables|Default|GetSniperUI))
  (bind _camera (Variables|Default|GetCamera))
  (:Started
    (UserInterface|Viewport|AddtoViewport _sniperui 0)
    (Camera|SetFieldOfView _camera 45.0))
  (:Completed
    (Widget|RemovefromParent _sniperui)
    (Camera|SetFieldOfView _camera 9e+01)))

(event Input|EnhancedActionEvents|EnhancedInputActionIA_HandGun
  (params (ActionValue :type Boolean) (ElapsedSeconds :type Float%20%28double-precision%29) (TriggeredSeconds :type Float%20%28double-precision%29) (InputAction :type Input%20Action%20Object%20Reference :default "/Game/Input/IA_HandGun.IA_HandGun"))
  (:Started
    (CallFunction|ChangeWeapon true)
    (bind _returnvalue (UserInterface|CreateWidget "/Game/Blueprint/WBP_CrosshairUI.WBP_CrosshairUI_C"))
    (UserInterface|Viewport|AddtoViewport _returnvalue 0))
  (:Completed
    (Widget|RemovefromParent _returnvalue)))

(event Input|EnhancedActionEvents|EnhancedInputActionIA_SniperGun
  (params (ActionValue :type Boolean) (ElapsedSeconds :type Float%20%28double-precision%29) (TriggeredSeconds :type Float%20%28double-precision%29) (InputAction :type Input%20Action%20Object%20Reference :default "/Game/Input/IA_SniperGun.IA_SniperGun"))
  (:Started
    (CallFunction|ChangeWeapon false)
    (bind _returnvalue (UserInterface|CreateWidget "/Game/Blueprint/WBP_SniperUI.WBP_SniperUI_C"))
    (Variables|Default|SetSniperUI _returnvalue)))

(event Input|EnhancedActionEvents|EnhancedInputActionIA_Run
  (params (ActionValue :type Boolean) (ElapsedSeconds :type Float%20%28double-precision%29) (TriggeredSeconds :type Float%20%28double-precision%29) (InputAction :type Input%20Action%20Object%20Reference :default "/Game/Input/IA_Run.IA_Run"))
  (bind _charactermovement (Variables|Character|GetCharacterMovement))
  (:Started
    (Variables|/Script/Engine.CharacterMovementComponent|SetMaxWalkSpeed _charactermovement 6e+02))
  (:Completed
    (Variables|/Script/Engine.CharacterMovementComponent|SetMaxWalkSpeed _charactermovement 3e+02)))

(event Input|EnhancedActionEvents|EnhancedInputActionIA_PlayerMove
  (params (ActionValue :type Vector%202D%20Structure) (ElapsedSeconds :type Float%20%28double-precision%29) (TriggeredSeconds :type Float%20%28double-precision%29) (InputAction :type Input%20Action%20Object%20Reference :default "/Game/Input/IA_PlayerMove.IA_PlayerMove"))
  (bind _returnvalue (Pawn|GetControlRotation :!class /Script/Engine.Pawn))
  (Pawn|Input|AddMovementInput (Math|Vector|GetRightVector (Math|Rotator|MakeRotator (.roll _returnvalue) 0.0 (.yaw _returnvalue))) (.x ActionValue) false)
  (Pawn|Input|AddMovementInput (Math|Vector|GetForwardVector (Math|Rotator|MakeRotator 0.0 0.0 (.yaw (Pawn|GetControlRotation :!class /Script/Engine.Pawn)))) (.y ActionValue) false))

(event Input|EnhancedActionEvents|EnhancedInputActionIA_LookUp
  (params (ActionValue :type Float%20%28double-precision%29) (ElapsedSeconds :type Float%20%28double-precision%29) (TriggeredSeconds :type Float%20%28double-precision%29) (InputAction :type Input%20Action%20Object%20Reference :default "/Game/Input/IA_LookUp.IA_LookUp"))
  (Pawn|Input|AddControllerPitchInput ActionValue))

(event Input|EnhancedActionEvents|EnhancedInputActionIA_Turn
  (params (ActionValue :type Float%20%28double-precision%29) (ElapsedSeconds :type Float%20%28double-precision%29) (TriggeredSeconds :type Float%20%28double-precision%29) (InputAction :type Input%20Action%20Object%20Reference :default "/Game/Input/IA_Turn.IA_Turn"))
  (Pawn|Input|AddControllerYawInput ActionValue))

(event Input|EnhancedActionEvents|EnhancedInputActionIA_PlayerJump
  (params (ActionValue :type Boolean) (ElapsedSeconds :type Float%20%28double-precision%29) (TriggeredSeconds :type Float%20%28double-precision%29) (InputAction :type Input%20Action%20Object%20Reference :default "/Game/Input/IA_PlayerJump.IA_PlayerJump"))
  (Character|Jump))

(event EventBeginPlay
  (Utilities|FlowControl|Sequence
    (:then_0
      (Collision|SetCollisionEnabled (Variables|Default|GetWeapon) "NoCollision")
      (Collision|SetCollisionEnabled (Variables|Default|GetSniper) "NoCollision"))
    (:then_1
      (Input|AddMappingContext (PlayerController|LocalPlayerSubsystems|GetEnhancedInputLocalPlayerSubsystem (Game|GetPlayerController 0)) "/Game/Input/IMC_Player.IMC_Player" 0 "(bIgnoreAllPressedKeysUntilRelease=True,bForceImmediately=False,bNotifyUserSettings=False)")
      (Variables|/Script/Engine.CharacterMovementComponent|SetMaxWalkSpeed (Variables|Character|GetCharacterMovement) 3e+02)
      (CallFunction|ChangeWeapon false))
    (:then_2
      (bind _returnvalue (UserInterface|CreateWidget "/Game/Blueprint/WBP_SniperUI.WBP_SniperUI_C"))
      (Variables|Default|SetSniperUI _returnvalue))))

(event Collision|EventActorBeginOverlap
  (params (OtherActor :type Actor%20Object%20Reference)))

(event EventTick
  (params (DeltaSeconds :type Float%20%28single-precision%29)))

(fn ConstructionScript)

(fn ChangeWeapon
  (params (bUsingHandGun :type Boolean))
  (Variables|Default|SetbUsing%20HandGun bUsingHandGun)
  (Rendering|SetVisibility (Variables|Default|GetWeapon) bUsingHandGun false)
  (Rendering|SetVisibility (Variables|Default|GetSniper) (not bUsingHandGun) false))

(fn HandGunFire
  (bind _weapon (Variables|Default|GetWeapon))
  (bind _returnvalue (Transformation|GetSocketTransform _weapon "FirePosition" "RTS_World"))
  (Game|SpawnActorfromClass "/Game/Blueprint/BP_Bullet.BP_Bullet_C" (Math|Transform|MakeTransform (.location _returnvalue) (.rotation _returnvalue) "0.250000,0.250000,0.250000") "AlwaysSpawn" "MultiplyWithRoot" 0 0)
  (Audio|PlaySound2D "/Game/Resource/HandGun.HandGun" 1.0 1.0 0.0 0 0))

(fn SniperFire
  (bind _sniper (Variables|Default|GetSniper))
  (bind _returnvalue (Transformation|GetSocketTransform _sniper "ShotPosition" "RTS_World"))
  (Game|SpawnActorfromClass "/Game/Blueprint/BP_Bullet.BP_Bullet_C" (Math|Transform|MakeTransform (.location _returnvalue) (.rotation _returnvalue) "0.250000,0.250000,0.250000") "AlwaysSpawn" "MultiplyWithRoot" 0 0)
  (Audio|PlaySound2D "/Game/Resource/SniperGun.SniperGun" 1.0 1.0 0.0 0 0))